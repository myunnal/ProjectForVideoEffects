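; BP_Canoe is an actor that moves a canoe mesh along a spline at a set speed.
; Each Tick advances a distance along the spline and places the mesh at that point, rotated to follow the spline with a -90 degree yaw offset.
; It also writes the RipplePoint world location to the BoatPosition parameter of the MPC_Water material parameter collection, exposing the boat position to water materials.
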(event `self.ReceiveTick`
  (params (DeltaSeconds :type "Float (single-precision)"))
  (bind _output_get (set `self.PositionOnSpline` (+ (* DeltaSeconds (`self.SpeedOnSpline`)) (`self.PositionOnSpline`) 0.0)))
  (`SceneComponent.K2_SetWorldLocation` (`self.StaticMesh`) (`SplineComponent.GetLocationAtDistanceAlongSpline` (`self.Spline`) _output_get "World") false false)
  (`SceneComponent.K2_SetWorldRotation` (`self.StaticMesh`) (`KismetMathLibrary.ComposeRotators` (`SplineComponent.GetRotationAtDistanceAlongSpline` (`self.Spline`) _output_get "World") (`KismetMathLibrary.MakeRotator` 0.0 0.0 -90.0)) false false)
  (`KismetMaterialLibrary.SetVectorParameterValue` "/Game/Materials/MPC_Water.MPC_Water" "BoatPosition" (`KismetMathLibrary.Conv_VectorToLinearColor` (`SceneComponent.K2_GetComponentLocation` (`self.RipplePoint`)))))

(fn `UserConstructionScript`)
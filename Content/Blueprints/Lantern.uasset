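; Lantern Blueprint that gently sways its root component to animate a hanging or swinging lantern.
; Each Tick sets the DefaultSceneRoot relative rotation from sine waves of game time.
; Roll and pitch each sum two sines of differing frequency for irregular motion, pitch at half strength, while yaw uses a single sine.
; The construction script is empty.
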(event `self.ReceiveTick`
  (params (DeltaSeconds :type "Float (single-precision)"))
  (`SceneComponent.K2_SetRelativeRotation` (`self.DefaultSceneRoot`) (`KismetMathLibrary.MakeRotator` (+ (* (`KismetMathLibrary.Sin` (* (`KismetSystemLibrary.GetGameTimeInSeconds`) 1.3)) 2.0) (`KismetMathLibrary.Sin` (* (`KismetSystemLibrary.GetGameTimeInSeconds`) 2.1))) (* (+ (* (`KismetMathLibrary.Sin` (* (`KismetSystemLibrary.GetGameTimeInSeconds`) 1.0)) 2.0) (`KismetMathLibrary.Sin` (* (`KismetSystemLibrary.GetGameTimeInSeconds`) 1.7))) 0.5) (`KismetMathLibrary.Sin` (* (`KismetSystemLibrary.GetGameTimeInSeconds`) 2.0))) false false))

(fn `UserConstructionScript`)
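; BP_SkyLantern is a sky lantern actor that floats upward while drifting back and forth.
; On Tick it accumulates time alive and adds a world offset scaled by frame delta time.
; A sine of that time, scaled by drift speed and amount, drives X and Y equally, giving a diagonal sway.
; Float speed alone sets the steady vertical movement.
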(event `self.ReceiveTick`
  (params (DeltaSeconds :type "Float (single-precision)"))
  ; Lantern dirfting/floating
  (bind _output_get (set `self.TimeAlive` (+ DeltaSeconds (`self.TimeAlive`))))
  (bind _returnvalue (* (* (`KismetMathLibrary.Sin` _output_get) (`self.DriftSpeed`)) (* (`GameplayStatics.GetWorldDeltaSeconds`) (`self.DriftAmount`))))
  (`self.K2_AddActorWorldOffset` (`KismetMathLibrary.MakeVector` _returnvalue _returnvalue (* (`GameplayStatics.GetWorldDeltaSeconds`) (`self.FloatSpeed`)))))

(fn `UserConstructionScript`)